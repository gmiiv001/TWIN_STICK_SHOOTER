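; Medkit pickup that heals a HeroCharacter over time when one overlaps it with Health below 100.
; The overlap stores the hero and starts a looping HealTheHero timer, which applies Delta through AffectHealth at a rate set by HealPerSecond.
; A DoOnce plays the attached healing sound and destroys the medkit five seconds later.
; The timer has no explicit stop, so healing runs until the actor is destroyed.
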(event Custom|HealTheHero
  (Default|AffectHealth (Variables|Default|GetHero) (Variables|Default|GetDelta)))

(event EventBeginPlay)

(event EventTick
  (params (DeltaSeconds :type Float%20%28single-precision%29)))

(event Collision|EventActorBeginOverlap
  (params (OtherActor :type Actor%20Object%20Reference))
  (bind _ashero_character (Utilities|Casting|CastToHeroCharacter OtherActor))
  (Variables|Default|SetHero _ashero_character)
  (if (< (Variables|/Script/TWIN_STICK_SHOOTER.BaseCharacter|GetHealth _ashero_character) 1e+02)
    (Utilities|Time|SetTimerbyFunctionName 0 "HealTheHero" (/ 1.0 (Variables|Default|GetHealPerSecond)) true)
    (Utilities|FlowControl|DoOnce false
      (:Completed
        (Audio|SpawnSoundAttached "/Game/Audio/Medkit_sound_hev-charger-half-life-2_01.Medkit_sound_hev-charger-half-life-2_01" (Variables|Default|GetHealingVolume) "None" "0, 0, 0" "0, 0, 0" "KeepRelativeOffset" false 1.0 1.0 0.0 0 0)
        (Utilities|FlowControl|Delay 5.0)
        (Actor|DestroyActor)))))

(fn ConstructionScript)